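; Player character component that shifts the camera's field of view with movement direction.
; On BeginPlay it caches the owning BP_PlayerCharacter and starts a looping timer for FovUpdate.
; Each update dots normalized velocity with actor forward, using the unclamped result to lerp between default and target FOV, regardless of speed.
; The camera moves toward that value via constant-rate interpolation, using frame delta time rather than the timer interval.
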(event Custom|FovUpdate
  (bind _character (Variables|Default|GetCharacter))
  (bind _camera (Variables|/Game/Blueprints/Character/Player/BP_PlayerCharacter.BP_PlayerCharacter_C|GetCamera _character))
  (Variables|Default|SetForwardAlpha (Math|Vector|DotProduct (Math|Vector|Normalize (Variables|/Script/Engine.MovementComponent|GetVelocity (Pawn|GetMovementComponent (Variables|Default|GetCharacter)))) (Transformation|GetActorForwardVector (Variables|Default|GetCharacter))))
  (Camera|SetFieldOfView _camera (Math|Interpolation|FInterptoConstant (Variables|/Script/Engine.CameraComponent|GetFieldOfView _camera) (Math|Float|Lerp (Variables|Default|GetFovDefault) (Variables|Default|GetFovTarget) (Variables|Default|GetForwardAlpha)) (Utilities|Time|GetWorldDeltaSeconds) (Variables|Default|GetInterp%20Speed))))

(event EventBeginPlay
  (bind _asbp_player_character (Utilities|Casting|CastToBP_PlayerCharacter (Components|GetOwner)))
  (Variables|Default|SetCharacter _asbp_player_character)
  (bind _returnvalue (Utilities|Time|SetTimerbyEvent (delegate Custom|FovUpdate) (Variables|Default|GetUpdateTimerTime) true))
  (Variables|Default|SetUpdateTimerHandle _returnvalue))

(event EventTick
  (params (DeltaSeconds :type Float%20%28single-precision%29)))