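; Level generator that builds the run as corridors of random room segments, starting at the start room and ending each in a safe room, or the last room after a set count.
; Each generation filters segments by unlocked ability requirements, then chains non-repeating picks at exit points.
; Delayed recursive events stagger spawning and signal completion.
; UnloadPreviousRooms destroys tracked older rooms one by one on a delay.
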(event Custom|UnloadNextSegment
  (if (not (Utilities|Array|IsEmpty (Variables|Default|GetRoomsScheduledForDeletion)))
    (Actor|DestroyActor (Utilities|Array|Get(acopy) (Variables|Default|GetRoomsScheduledForDeletion)))
    (Utilities|Array|RemoveIndex (Variables|Default|GetRoomsScheduledForDeletion))
    (Utilities|FlowControl|Delay 0.5)
    (CallFunction|UnloadNextSegment)))

(event Custom|BuildNextSegment
  (params (AttachmentPoint :type Arrow%20Component%20Object%20Reference) (SegmentsLeft :type Integer))
  (bind _outroomsegment (CallFunction|AttachRandomRoom AttachmentPoint))
  (Utilities|Array|Add (Variables|Default|GetOldRooms) _outroomsegment)
  (Utilities|FlowControl|Delay 0.1)
  (if (> SegmentsLeft 1)
    (CallFunction|BuildNextSegment (Variables|/Game/Blueprints/Level/BP_RoomSegment.BP_RoomSegment_C|GetExitPoint _outroomsegment) (- SegmentsLeft 1))
    (else
      (CallFunction|AttachSafeZone (Variables|/Game/Blueprints/Level/BP_RoomSegment.BP_RoomSegment_C|GetExitPoint _outroomsegment))
      (Utilities|FlowControl|Delay 2.0)
      (Default|CallOnFinishedGenerating))))

(event EventBeginPlay
  (bind _outactors (Actor|GetAllActorsOfClass "/Game/Blueprints/Level/BP_StartRoom.BP_StartRoom_C"))
  (bind _output_get (Variables|Default|SetStartRoom (Utilities|Array|Get(acopy) _outactors)))
  (Utilities|Array|Add (Variables|Default|GetOldRooms) _output_get)
  (CallFunction|GenerateSegmentfromSafeZone (Variables|/Game/Blueprints/Level/BP_StartRoom.BP_StartRoom_C|GetCorridorPoint _output_get)))

(fn ConstructionScript)

(fn GetFilteredRooms
  (params (FilterAbility :type BP%20Movement%20Data%20Asset%20Object%20Reference))
  (Utilities|FlowControl|Sequence
    (:then_0
      (Utilities|IsValid FilterAbility
        (:Is%20Valid
          (Utilities|Array|Add (LocalVariables|GetUnlockedAbilities) (Variables|/Game/DataAssets/Base/BP_BaseUpgradeDataAsset.BP_BaseUpgradeDataAsset_C|GetId FilterAbility)))))
    (:then_1
      (for _array_element (Variables|Default|GetRoomSegments)
        (LocalVariables|SetIsViable true)
        (bind _array_element_2 (Utilities|Array|ForEachLoopwithBreak (.RequiredAbilities (Utilities|GetClassDefaults _array_element)) :!label _label)
          (:LoopBody
            (if (not (Utilities|Array|ContainsItem (LocalVariables|GetUnlockedAbilities) (Variables|/Game/DataAssets/Base/BP_MovementDataAsset.BP_MovementDataAsset_C|GetId (Utilities|ResolveSoftReference _array_element_2))))
              (LocalVariables|SetIsViable false)
              (goto _label Break)))
          (:Completed
            (if (LocalVariables|GetIsViable)
              (Utilities|Array|Add (LocalVariables|GetFilteredRoomSegments) _array_element)))))
      (return (LocalVariables|GetFilteredRoomSegments)))))

(fn AttachRandomRoom
  (params (AttachmentPoint :type Arrow%20Component%20Object%20Reference))
  (bind _output_get (LocalVariables|SetSelectedRandomRoom (.OutItem (Utilities|Array|Random (Variables|Default|GetFilteredRooms)))))
  (bind _returnvalue (Game|SpawnActorfromClass _output_get (Math|Transform|MakeTransform (Transformation|GetWorldLocation AttachmentPoint) (Transformation|GetWorldRotation AttachmentPoint) "1.000000,1.000000,1.000000") "AlwaysSpawn" "MultiplyWithRoot" 0 0))
  (Utilities|Array|RemoveItem (Variables|Default|GetFilteredRooms) (LocalVariables|GetSelectedRandomRoom))
  (return _returnvalue))

(fn BuildCorridor
  (params (LengthFrom :type Integer) (LengthTo :type Integer) (FromAttachmentPoint :type Arrow%20Component%20Object%20Reference))
  (CallFunction|BuildNextSegment FromAttachmentPoint (Math|Random|RandomIntegerinRange LengthFrom LengthTo))
  (return))

(fn AttachSafeZone
  (params (AttachmentPoint :type Arrow%20Component%20Object%20Reference))
  (if (!= (Variables|Default|GetCurrentSafeRoomIndex) (Variables|Default|GetSafeZonesUntilLastRoom))
    (bind _returnvalue (Game|SpawnActorfromClass "/Game/Blueprints/Level/BP_SafeRoomModeled.BP_SafeRoomModeled_C" (Math|Transform|MakeTransform (Transformation|GetWorldLocation AttachmentPoint) (Transformation|GetWorldRotation AttachmentPoint) "1.000000,1.000000,1.000000") "AlwaysSpawn" "MultiplyWithRoot" 0 (Variables|Default|GetCurrentSafeRoomIndex) 0))
    (LocalVariables|SetNewSafeZone _returnvalue)
    (Math|Integer|IncrementInt (Variables|Default|GetCurrentSafeRoomIndex)
      (:%20%20
        (return (LocalVariables|GetNewSafeZone))))
    (else
      (Game|SpawnActorfromClass "/Game/Blueprints/Level/BP_LastRoom.BP_LastRoom_C" (Math|Transform|MakeTransform (Transformation|GetWorldLocation AttachmentPoint) (Transformation|GetWorldRotation AttachmentPoint) "1.000000,1.000000,1.000000") "AlwaysSpawn" "MultiplyWithRoot" 0 0)
      (return 0))))

(fn GenerateSegmentfromSafeZone
  (params (AttachmentPoint :type Arrow%20Component%20Object%20Reference) (FilterAbility :type BP%20Movement%20Data%20Asset%20Object%20Reference))
  (bind _result (CallFunction|GetFilteredRooms FilterAbility))
  (bind _output_get (Variables|Default|SetFilteredRooms _result))
  (CallFunction|BuildCorridor (Variables|Default|GetRoomSegmentsFrom) (Math|Integer|Min(Integer) (Utilities|Array|Length _output_get) (Variables|Default|GetRoomSegmentsTo)) AttachmentPoint)
  (return))

(fn UnloadPreviousRooms
  (Variables|Default|SetRoomsScheduledForDeletion (Variables|Default|GetOldRooms))
  (Utilities|Array|Clear (Variables|Default|GetOldRooms))
  (CallFunction|UnloadNextSegment))