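; Double sliding gate prop with left and right door components, exposing OpenDoor and CloseDoor events.
; A single timeline drives each door's relative Y position at a fixed height, playing from the start to open and reversing from the end to close.
; On BeginPlay, IsOpen offsets the doors apart instantly to start the gate open; the open and close events never update that flag.
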(event Custom|OpenDoor
  (bind (_direction _rightdoorpos _leftdoorpos) (Timeline|OpenDoorTimeline PlayFromStart)
    (:Update
      (Utilities|FlowControl|Sequence
        (:then_0
          (Transformation|SetRelativeLocation (Variables|Default|GetRightDoor) (Math|Vector|MakeVector 0.0 _rightdoorpos 1.5e+02) false false))
        (:then_1
          (Transformation|SetRelativeLocation (Variables|Default|GetLeftDoor) (Math|Vector|MakeVector 0.0 _leftdoorpos 1.5e+02) false false))))))

(event Custom|CloseDoor
  (bind (_direction _rightdoorpos _leftdoorpos) (Timeline|OpenDoorTimeline ReverseFromEnd)
    (:Update
      (Utilities|FlowControl|Sequence
        (:then_0
          (Transformation|SetRelativeLocation (Variables|Default|GetRightDoor) (Math|Vector|MakeVector 0.0 _rightdoorpos 1.5e+02) false false))
        (:then_1
          (Transformation|SetRelativeLocation (Variables|Default|GetLeftDoor) (Math|Vector|MakeVector 0.0 _leftdoorpos 1.5e+02) false false))))))

(event EventBeginPlay
  (if (Variables|Default|GetIsOpen)
    (Transformation|AddRelativeLocation (Variables|Default|GetRightDoor) "0.000000,90.000000,0.000000" false true)
    (Transformation|AddRelativeLocation (Variables|Default|GetLeftDoor) "0.000000,-90.000000,0.000000" false true)))

(fn ConstructionScript)