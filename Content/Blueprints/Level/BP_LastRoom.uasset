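; BP_LastRoom is the final room actor, whose exit trigger ends the run with a win.
; When the player character overlaps ExitTrigger, it keeps the lower of the overall timer and best timer in the experience component, then saves the game.
; It then creates WB_WinScreen with both times and shows it through the player controller's MenuLayer, paused and not closable by key.
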(event OnComponentBeginOverlap(ExitTrigger)
  (params (OverlappedComponent :type Primitive%20Component%20Object%20Reference) (OtherActor :type Actor%20Object%20Reference) (OtherComp :type Primitive%20Component%20Object%20Reference) (OtherBodyIndex :type Integer) (bFromSweep :type Boolean) (SweepResult :type Hit%20Result%20Structure%20%28by%20ref%29))
  (bind _asbp_player_character (Utilities|Casting|CastToBP_PlayerCharacter OtherActor))
  (Variables|/Game/Blueprints/Character/Player/BP_ExperienceComponent.BP_ExperienceComponent_C|SetOverallBestTimer (Variables|/Game/Blueprints/Character/Player/BP_PlayerCharacter.BP_PlayerCharacter_C|GetBP_ExperienceComponent _asbp_player_character) (Math|Float|Min(Float) (Variables|/Game/Blueprints/Character/Player/BP_ExperienceComponent.BP_ExperienceComponent_C|GetOverallTimer (Variables|/Game/Blueprints/Character/Player/BP_PlayerCharacter.BP_PlayerCharacter_C|GetBP_ExperienceComponent _asbp_player_character)) (Variables|/Game/Blueprints/Character/Player/BP_ExperienceComponent.BP_ExperienceComponent_C|GetOverallBestTimer (Variables|/Game/Blueprints/Character/Player/BP_PlayerCharacter.BP_PlayerCharacter_C|GetBP_ExperienceComponent _asbp_player_character))))
  (Default|SaveGame _asbp_player_character)
  (bind _asbp_player_controller (Utilities|Casting|CastToBP_PlayerController (Game|GetPlayerController 0)))
  (bind _returnvalue (UserInterface|CreateWidget "/Game/Blueprints/UI/WB_WinScreen.WB_WinScreen_C" 0 (Variables|/Game/Blueprints/Character/Player/BP_ExperienceComponent.BP_ExperienceComponent_C|GetOverallTimer (Variables|/Game/Blueprints/Character/Player/BP_PlayerCharacter.BP_PlayerCharacter_C|GetBP_ExperienceComponent _asbp_player_character)) (Variables|/Game/Blueprints/Character/Player/BP_ExperienceComponent.BP_ExperienceComponent_C|GetOverallBestTimer (Variables|/Game/Blueprints/Character/Player/BP_PlayerCharacter.BP_PlayerCharacter_C|GetBP_ExperienceComponent _asbp_player_character))))
  (Default|SetCurrentMenu (Variables|/Game/Blueprints/Character/Player/BP_PlayerController.BP_PlayerController_C|GetMenuLayer _asbp_player_controller) _returnvalue true false))

(event EventBeginPlay)

(event Collision|EventActorBeginOverlap
  (params (OtherActor :type Actor%20Object%20Reference)))

(event EventTick
  (params (DeltaSeconds :type Float%20%28single-precision%29)))

(fn ConstructionScript)