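; BP_CorridorEntranceDoor is an interactable safe zone door that generates a new level segment, filtered by its assigned movement ability, before opening.
; Interacting while closed and unblocked has BP_LevelGenerator build from the door's attachment point and blocks all doors in the parent BP_SafeZone.
; When generation finishes, the child BP_Gate opens.
; AssignAbility shows the ability's image through a dynamic decal material and toggles the plane's visibility.
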(event Custom|OnFinishedGenerating
  (bind _asbp_gate (Utilities|Casting|CastToBP_Gate (Variables|/Script/Engine.ChildActorComponent|GetChildActor (Variables|Default|GetGate))))
  (Default|OpenDoor _asbp_gate)
  (EventDispatchers|UnbindEventfromOnFinishedGenerating (Variables|Default|GetLevelGenerator) (delegate Custom|OnFinishedGenerating))
  (Variables|Default|SetIsOpen true))

(event EventInteract
  (if (and (not (Variables|Default|GetIsOpen)) (not (Variables|Default|GetIsBlocked)))
    (bind _outactors (Actor|GetAllActorsOfClass "/Game/Blueprints/Level/BP_LevelGenerator.BP_LevelGenerator_C"))
    (bind _output_get (Variables|Default|SetLevelGenerator (Utilities|Array|Get(acopy) _outactors)))
    (Default|GenerateSegmentfromSafeZone _output_get (Variables|Default|GetAttachmentPoint) (Variables|Default|GetMovementAbility))
    (EventDispatchers|BindEventtoOnFinishedGenerating _output_get (EventDispatchers|CreateEvent :!event Custom|OnFinishedGenerating))
    (bind _asbp_safe_zone (Utilities|Casting|CastToBP_SafeZone (Actor|GetParentActor)))
    (Default|SetBlockedforAllDoors _asbp_safe_zone true)))

(fn ConstructionScript)

(fn AssignAbility
  (params (Ability :type BP%20Movement%20Data%20Asset%20Object%20Reference))
  (bind _output_get (Variables|Default|SetMovementAbility Ability))
  (Utilities|IsValid _output_get
    (:Is%20Valid
      (Rendering|SetVisibility (Variables|Default|GetPlane) true true)
      (bind _returnvalue (Rendering|Material|CreateDynamicMaterialInstance (Variables|Default|GetDecal) :!class /Script/Engine.DecalComponent))
      (Rendering|Material|SetTextureParameterValue _returnvalue "Image" (Variables|/Game/DataAssets/Base/BP_BaseUpgradeDataAsset.BP_BaseUpgradeDataAsset_C|GetImage _output_get)))
    (:Is%20Not%20Valid
      (Rendering|SetVisibility (Variables|Default|GetPlane) false true))))

(fn CanInteract
  (return (and (not (Variables|Default|GetIsOpen)) (not (Variables|Default|GetIsBlocked)))))