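; BP_SkillBook is a one-time interactable book that grants the player new abilities.
; A looping timeline moves the book component relative to its starting position until it is collected.
; On Interact it adds time machine energy to BP_PlayerCharacter, has BP_PlayerController unlock new abilities, then destroys the book and stops the animation.
; It also notifies its SafeZone reference that the book was used, and CanInteract reports availability.
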(event EventBeginPlay
  (bind _bookforskills (Variables|Default|GetBookForSkills))
  (Variables|Default|SetBaseRelativeLocation (Variables|/Script/Engine.SceneComponent|GetRelativeLocation (Variables|Default|GetBookForSkills)))
  (bind _position (Timeline|BookMoveAnimation Play)
    (:Update
      (Utilities|IsValid _bookforskills
        (:Is%20Valid
          (Transformation|SetRelativeLocation _bookforskills (+ _position (Variables|Default|GetBaseRelativeLocation)) false false))))
    (:Finished
      (Utilities|FlowControl|Delay 0.0)
      (Timeline|BookMoveAnimation PlayFromStart))))

(event EventInteract
  (bind _bookforskills (Variables|Default|GetBookForSkills))
  (if (Variables|Default|GetIsAvailable)
    (Utilities|FlowControl|Sequence
      (:then_0
        (Variables|Default|SetIsAvailable false)
        (bind _asbp_player_character (Utilities|Casting|CastToBP_PlayerCharacter (Game|GetPlayerCharacter 0)))
        (Default|AddTimeMachineEnergy _asbp_player_character 1e+01)
        (bind _asbp_player_controller (Utilities|Casting|CastToBP_PlayerController (Game|GetPlayerController 0)))
        (Default|UnlockNewAbilities _asbp_player_controller)
        (Components|DestroyComponent (Variables|Default|GetBookForSkills))
        (bind _position (Timeline|BookMoveAnimation Stop)
          (:Update
            (Utilities|IsValid _bookforskills
              (:Is%20Valid
                (Transformation|SetRelativeLocation _bookforskills (+ _position (Variables|Default|GetBaseRelativeLocation)) false false))))
          (:Finished
            (Utilities|FlowControl|Delay 0.0)
            (Timeline|BookMoveAnimation PlayFromStart))))
      (:then_1
        (Default|OnSkillBookUsed (Variables|Default|GetSafeZone))))))

(fn ConstructionScript)

(fn CanInteract
  (return (Variables|Default|GetIsAvailable)))