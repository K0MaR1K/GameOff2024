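; Player component that tracks time spent outside safe zones and awards experience for how quickly each room is completed.
; Tick advances per-room and overall timers while the player is outside a safe zone, broadcasting both.
; Entering a new room or safe zone converts room time into experience scaled by target time and room difficulty, then resets the room timer.
; Experience gains can trigger multiple level-ups, with each level's requirement growing progressively.
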(event Custom|OnEnterNewRoom
  (params (WasInsideSafeZone :type Boolean) (Room :type BP%20Room%20Segment%20Object%20Reference))
  (Utilities|FlowControl|Sequence
    (:then_0
      (if (not WasInsideSafeZone)
        (CallFunction|AddExperiencefromRoomTime (Variables|RoomTimer|GetRoomTimer) (Variables|/Game/Blueprints/Level/BP_RoomSegment.BP_RoomSegment_C|GetRoomDifficulty Room))))
    (:then_1
      (Variables|RoomTimer|SetRoomTimer 0.0))))

(event Custom|OnEnterSafeZone
  (params (LastRoom :type BP%20Room%20Segment%20Object%20Reference))
  (CallFunction|AddExperiencefromRoomTime (Variables|RoomTimer|GetRoomTimer) (Variables|/Game/Blueprints/Level/BP_RoomSegment.BP_RoomSegment_C|GetRoomDifficulty LastRoom))
  (Variables|RoomTimer|SetRoomTimer 0.0))

(event EventTick
  (params (DeltaSeconds :type Float%20%28single-precision%29))
  (if (not (Variables|/Game/Blueprints/Character/Player/BP_PlayerCharacter.BP_PlayerCharacter_C|GetIsInsideSafeZone (Variables|Default|GetPlayerCharacter)))
    (Utilities|FlowControl|Sequence
      (:then_0
        (bind _output_get (Variables|RoomTimer|SetRoomTimer (+ (Variables|RoomTimer|GetRoomTimer) DeltaSeconds)))
        (Default|CallOnRoomTimerUpdated _output_get))
      (:then_1
        (bind _output_get_2 (Variables|Default|SetOverallTimer (+ DeltaSeconds (Variables|Default|GetOverallTimer))))
        (Default|CallOnOverallTimerUpdated _output_get_2)))))

(event EventBeginPlay
  (bind _asbp_player_character (Utilities|Casting|CastToBP_PlayerCharacter (Components|GetOwner)))
  (Variables|Default|SetPlayerCharacter _asbp_player_character))

(fn AddExperiencefromRoomTime
  (params (RoomCompletionTime :type Float%20%28double-precision%29) (RoomDifficulty :type Float%20%28double-precision%29))
  (CallFunction|AddExperience (* (/ (Variables|RoomTimer|GetTargetRoomCompletionTime) RoomCompletionTime) (Variables|Experience|GetExperienceForTargetCompletion) RoomDifficulty)))

(fn AddExperience
  (params (Amount :type Float%20%28double-precision%29))
  (Variables|Experience|SetCurrentExperience (+ Amount (Variables|Experience|GetCurrentExperience)))
  (while (> (Variables|Experience|GetCurrentExperience) (Variables|Experience|GetExperienceForNextLevel))
    (Math|Integer|IncrementInt (Variables|Default|GetCurrentLevel)
      (:%20%20
        (Variables|Experience|SetExperienceForPreviousLevel (Variables|Experience|GetExperienceForNextLevel))
        (Variables|Experience|SetExperienceForNextLevel (+ (Variables|Experience|GetExperienceForNextLevel) (Variables|Experience|GetAdditionalExperiencePerLevel)))
        (Variables|Experience|SetAdditionalExperiencePerLevel (+ (Variables|Experience|GetAdditionalExperiencePerLevel) 5e+02))
        (Default|CallOnLevelUp (Variables|Default|GetCurrentLevel)))))
  (Default|CallOnExperienceAdded Amount))