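; BP_ShootingComponent is a player component that handles firing the rifle and destroying turrets.
; On the shoot input, a DoOnce fires the child-actor rifle and resets after a short delay, limiting fire rate.
; It sphere-traces forward from the camera and spawns an explosion emitter at the trace result.
; A hit Turret is destroyed and a turret-evade lore note unlocks through the player's lore component.
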(event Input|EnhancedActionEvents|EnhancedInputActionIA_Shoot
  (params (ActionValue :type Boolean) (ElapsedSeconds :type Float%20%28double-precision%29) (TriggeredSeconds :type Float%20%28double-precision%29) (InputAction :type Input%20Action%20Object%20Reference :default "/Game/Input/IA_Shoot.IA_Shoot"))
  (bind _playercharacter (Variables|Default|GetPlayerCharacter))
  (bind _camera (Variables|/Game/Blueprints/Character/Player/BP_PlayerCharacter.BP_PlayerCharacter_C|GetCamera _playercharacter))
  (bind _returnvalue (Transformation|GetWorldLocation _camera))
  (:Started
    (Utilities|FlowControl|DoOnce false :!label _label
      (:Completed
        (bind _asbp_rifle (Utilities|Casting|CastToBP_Rifle (Variables|/Script/Engine.ChildActorComponent|GetChildActor (Variables|/Game/Blueprints/Character/Player/BP_PlayerCharacter.BP_PlayerCharacter_C|GetBP_Rifle (Variables|Default|GetPlayerCharacter)))))
        (Default|Shoot _asbp_rifle)
        (Utilities|FlowControl|Sequence
          (:then_0
            (Utilities|FlowControl|Delay 1.5)
            (goto _label Reset))
          (:then_1
            (bind _outhit (Collision|SphereTraceByChannel _returnvalue (+ _returnvalue (* (Math|Vector|GetForwardVector (Transformation|GetWorldRotation _camera)) 5e+03)) 1e+01 "TraceTypeQuery1" false 0 "None"))
            (Effects|SpawnEmitteratLocation "/Game/StarterContent/Particles/P_Explosion.P_Explosion" (.location _outhit) (Math|Conversions|RotationFromXVector (.normal _outhit)))
            (bind _asturret (Utilities|Casting|CastToTurret (.hitactor _outhit)))
            (Actor|DestroyActor _asturret)
            (Default|UnlockNote (Variables|/Game/Blueprints/Character/Player/BP_PlayerCharacter.BP_PlayerCharacter_C|GetBP_LoreComponent (Variables|Default|GetPlayerCharacter)) "/Game/DataAssets/Notes/DA_PlayerNote_TurretEvade.DA_PlayerNote_TurretEvade")))))))

(event EventBeginPlay
  (bind _asbp_player_character (Utilities|Casting|CastToBP_PlayerCharacter (Components|GetOwner)))
  (Variables|Default|SetPlayerCharacter _asbp_player_character))

(event EventTick
  (params (DeltaSeconds :type Float%20%28single-precision%29)))