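; Player character component that detects interactable actors in view and triggers interaction with them.
; A looping timer line-traces from the camera along the control rotation and caches any hit actor implementing BPI_InteractInterface.
; An event dispatcher fires when focus turns on for a target passing CanInteract, or off when none is hit.
; The IA_Interact input calls Interact on the cached target without rechecking CanInteract.
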(event Custom|CheckInteract
  (bind _playercharacter (Variables|Default|GetPlayerCharacter))
  (bind _camera (Variables|/Game/Blueprints/Character/Player/BP_PlayerCharacter.BP_PlayerCharacter_C|GetCamera _playercharacter))
  (bind _returnvalue (Transformation|GetWorldLocation _camera))
  (bind (_outhit _returnvalue_2) (Collision|LineTraceByChannel _returnvalue (+ _returnvalue (* (Math|Vector|GetForwardVector (Pawn|GetControlRotation _playercharacter :!class /Script/Engine.Pawn)) 5e+02)) "TraceTypeQuery1" false 0 "None" true "(R=1.000000,G=0.000000,B=0.000000,A=1.000000)" "(R=0.000000,G=1.000000,B=0.000000,A=1.000000)" 0.1))
  (if _returnvalue_2
    (if (Utilities|DoesObjectImplementInterface (.hitactor _outhit) "/Game/Blueprints/Level/Interactables/BPI_InteractInterface.BPI_InteractInterface_C")
      (bind _asbpi_interact_interface (Utilities|Casting|CastToBPI_InteractInterface (.hitactor _outhit)))
      (bind _output_get (Variables|Default|SetInteractable _asbpi_interact_interface))
      (bind _result (Default|CanInteract _output_get))
      (if _result
        (if (not (Variables|Default|GetIsInteracting))
          (bind _output_get_2 (Variables|Default|SetIsInteracting true))
          (Default|CallOnInteractingChanged _output_get_2)))
      (else
        (Variables|Default|SetInteractable 0 :!label _label)
        (if (Variables|Default|GetIsInteracting)
          (bind _output_get_3 (Variables|Default|SetIsInteracting false))
          (Default|CallOnInteractingChanged _output_get_3))))
    (else
      (goto _label))))

(event Input|EnhancedActionEvents|EnhancedInputActionIA_Interact
  (params (ActionValue :type Boolean) (ElapsedSeconds :type Float%20%28double-precision%29) (TriggeredSeconds :type Float%20%28double-precision%29) (InputAction :type Input%20Action%20Object%20Reference :default "/Game/Input/IA_Interact.IA_Interact"))
  (bind _interactable (Variables|Default|GetInteractable))
  (:Started
    (if (Utilities|IsValidInterface _interactable)
      (Default|Interact _interactable))))

(event EventBeginPlay
  (Utilities|Time|SetTimerbyEvent (delegate Custom|CheckInteract) 0.1 true)
  (bind _asbp_player_character (Utilities|Casting|CastToBP_PlayerCharacter (Components|GetOwner)))
  (Variables|Default|SetPlayerCharacter _asbp_player_character))