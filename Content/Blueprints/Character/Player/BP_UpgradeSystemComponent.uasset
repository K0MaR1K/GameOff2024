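; Player upgrade component that banks an upgrade point on each level-up and tracks which upgrades and movement abilities the player owns.
; At BeginPlay it indexes the upgrade list by Id; applying one sets movement abilities to owned or increments other upgrades, then broadcasts it.
; Random offers draw without repeats from upgrades passing level, dependency and ability-versus-regular checks.
; It can also pick a random unlocked ability, excluding double jump.
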(event Custom|OnLevelUp
  (params (NewLevel :type Integer))
  (bind _result (Math|Integer|IncrementInt (Variables|Default|GetUpgradesAvailable))
    (:%20%20
      (Default|CallOnUpgradesAmountChanged _result))))

(event EventBeginPlay
  (bind _asbp_player_character (Utilities|Casting|CastToBP_PlayerCharacter (Components|GetOwner)))
  (bind _output_get (Variables|Default|SetPlayerCharacter _asbp_player_character))
  (EventDispatchers|BindEventtoOnLevelUp (Variables|/Game/Blueprints/Character/Player/BP_PlayerCharacter.BP_PlayerCharacter_C|GetBP_ExperienceComponent _output_get) (EventDispatchers|CreateEvent :!event Custom|OnLevelUp))
  (for _array_element (Variables|Default|GetUpgradesCompleteList)
    (Utilities|Map|Add (Variables|Default|GetUpgradesAmountMap) (Variables|/Game/DataAssets/Base/BP_BaseUpgradeDataAsset.BP_BaseUpgradeDataAsset_C|GetId _array_element) 0)
    (Utilities|Map|Add (Variables|Default|GetIdToUpgradeMap) (Variables|/Game/DataAssets/Base/BP_BaseUpgradeDataAsset.BP_BaseUpgradeDataAsset_C|GetId _array_element) _array_element)))

(fn ApplyUpgrade
  (params (Id :type String))
  (LocalVariables|SetUpgradeToUnlock (.Value (Utilities|Map|Find (Variables|Default|GetIdToUpgradeMap) Id)))
  (Utilities|FlowControl|Sequence
    (:then_0
      (Utilities|Casting|CastToBP_MovementDataAsset (LocalVariables|GetUpgradeToUnlock)
        (:then
          (LocalVariables|SetValueToSet 1))
        (:CastFailed
          (LocalVariables|SetValueToSet (+ (.Value (Utilities|Map|Find (Variables|Default|GetUpgradesAmountMap) Id)) 1)))))
    (:then_1
      (Utilities|Map|Add (Variables|Default|GetUpgradesAmountMap) Id (LocalVariables|GetValueToSet))
      (Default|CallOnUpgradeApplied (LocalVariables|GetUpgradeToUnlock) (LocalVariables|GetValueToSet)))))

(fn GetRandomUpgrades
  (params (Amount :type Integer) (IsAbilityUnlock :type Boolean))
  (Utilities|FlowControl|Sequence
    (:then_0
      (for _array_element (Variables|Default|GetUpgradesCompleteList)
        (bind _result (CallFunction|IsUpgradeAvailable _array_element IsAbilityUnlock))
        (if _result
          (Utilities|Array|Add (LocalVariables|GetCurrentUpgradePool) _array_element))))
    (:then_1
      (for _index (range 1 Amount)
        (bind _output_get (LocalVariables|SetRandomlySelectedUpgrade (.OutItem (Utilities|Array|Random (LocalVariables|GetCurrentUpgradePool)))))
        (Utilities|Array|Add (LocalVariables|GetSelectedUpgrades) _output_get)
        (Utilities|Array|RemoveItem (LocalVariables|GetCurrentUpgradePool) _output_get))
      (return (LocalVariables|GetSelectedUpgrades)))))

(fn IsUpgradeAvailable
  (params (Upgrade :type BP%20Base%20Upgrade%20Data%20Asset%20Object%20Reference) (IsAbilityUnlock :type Boolean))
  (if (>= (Variables|/Game/Blueprints/Character/Player/BP_ExperienceComponent.BP_ExperienceComponent_C|GetCurrentLevel (Variables|/Game/Blueprints/Character/Player/BP_PlayerCharacter.BP_PlayerCharacter_C|GetBP_ExperienceComponent (Variables|Default|GetPlayerCharacter))) (Variables|/Game/DataAssets/Base/BP_BaseUpgradeDataAsset.BP_BaseUpgradeDataAsset_C|GetRequiredLevel Upgrade))
    (Utilities|FlowControl|Sequence
      (:then_0
        (bind _asbp_movement_data_asset (Utilities|Casting|CastToBP_MovementDataAsset Upgrade)
          (:then
            (if IsAbilityUnlock
              (if (== (.Value (Utilities|Map|Find (Variables|Default|GetUpgradesAmountMap) (Variables|/Game/DataAssets/Base/BP_BaseUpgradeDataAsset.BP_BaseUpgradeDataAsset_C|GetId _asbp_movement_data_asset))) 1)
                (return false))
              (else
                (return false))))
          (:CastFailed
            (if IsAbilityUnlock
              (return false)))))
      (:then_1
        (for _array_element (Variables|/Game/DataAssets/Base/BP_BaseUpgradeDataAsset.BP_BaseUpgradeDataAsset_C|GetDependencies Upgrade)
          (if (== (.Value (Utilities|Map|Find (Variables|Default|GetUpgradesAmountMap) (Variables|/Game/DataAssets/Base/BP_BaseUpgradeDataAsset.BP_BaseUpgradeDataAsset_C|GetId _array_element))) 0)
            (return false)))
        (return true)))
    (else
      (return false))))

(fn UseUpgrade
  (bind _result (Math|Integer|DecrementInt (Variables|Default|GetUpgradesAvailable))
    (:%20%20
      (Default|CallOnUpgradesAmountChanged _result))))

(fn GetRandomUnlockedAbility
  (bind _keys (Utilities|Map|Keys (Variables|Default|GetUpgradesAmountMap)))
  (for _array_element _keys
    (if (Utilities|Enum|NotEqual(Enum) _array_element "double_jump")
      (bind _asbp_movement_data_asset (Utilities|Casting|CastToBP_MovementDataAsset (.Value (Utilities|Map|Find (Variables|Default|GetIdToUpgradeMap) _array_element))))
      (if (== (.Value (Utilities|Map|Find (Variables|Default|GetUpgradesAmountMap) _array_element)) 1)
        (Utilities|Array|Add (LocalVariables|GetTempList) _asbp_movement_data_asset))))
  (Utilities|Array|Add (LocalVariables|GetTempList) 0)
  (return (.OutItem (Utilities|Array|Random (LocalVariables|GetTempList)))))