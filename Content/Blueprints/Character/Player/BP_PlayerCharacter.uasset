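; Player character for a room-based movement game with health, unlockable movement abilities and time-machine energy.
; Upgrades scale CharacterMovement stats or unlock movement components by ID, while Tick handles curve-driven friction, slide and footstep audio, and health regen.
; Death or falling returns the player to the room start and costs energy, which also drains outside safe zones.
; Running out on such a penalty saves notes, best time and death flag, then reloads MainMap.
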(event OnUpgradeApplied(BP_UpgradeSystemComponent)
  (params (Upgrade :type BP%20Base%20Upgrade%20Data%20Asset%20Object%20Reference) (NewValue :type Integer))
  ;[1 1 1] Apply Upgrades
  (bind _asbp_parameter_upgrade_data_asset (Utilities|Casting|CastToBP_ParameterUpgradeDataAsset Upgrade)
    (:then
      (Variables|Default|SetCurrentUpgradesAmount NewValue)
      (bind _output_get (Variables|Default|SetCurrentUpgradeToApply _asbp_parameter_upgrade_data_asset))
      (switch string (Variables|/Game/DataAssets/Base/BP_BaseUpgradeDataAsset.BP_BaseUpgradeDataAsset_C|GetId _output_get)
        (:move_speed
          (Variables|/Script/Engine.CharacterMovementComponent|SetMaxWalkSpeed (Variables|Character|GetCharacterMovement) (Default|CalculateUpgradedValue (Variables|Default|GetCurrentUpgradeToApply) (Variables|Default|GetCurrentUpgradesAmount) (Variables|DefaultUpgradeValues|GetDefaultMaxWalkSpeed))))
        (:acceleration
          (Variables|/Script/Engine.CharacterMovementComponent|SetMaxAcceleration (Variables|Character|GetCharacterMovement) (Default|CalculateUpgradedValue (Variables|Default|GetCurrentUpgradeToApply) (Variables|Default|GetCurrentUpgradesAmount) (Variables|DefaultUpgradeValues|GetDefaultAcceleration))))
        (:air_control
          (Variables|/Script/Engine.CharacterMovementComponent|SetAirControl (Variables|Character|GetCharacterMovement) (Default|CalculateUpgradedValue (Variables|Default|GetCurrentUpgradeToApply) (Variables|Default|GetCurrentUpgradesAmount) (Variables|DefaultUpgradeValues|GetDefaultAirControl))))
        (:jump_height
          (Variables|/Script/Engine.CharacterMovementComponent|SetJumpZVelocity (Variables|Character|GetCharacterMovement) (Default|CalculateUpgradedValue (Variables|Default|GetCurrentUpgradeToApply) (Variables|Default|GetCurrentUpgradesAmount) (Variables|DefaultUpgradeValues|GetDefaultJumpVelocity))))))
    (:CastFailed
      (CallFunction|UnlockMovementAbility (Variables|/Game/DataAssets/Base/BP_BaseUpgradeDataAsset.BP_BaseUpgradeDataAsset_C|GetId Upgrade)))))

(event Custom|DashTriggered
  ;[1 1 1] Sound
  (Utilities|PlaySound(else->) 0.0 "/Game/Sound/SFX/dash.dash" true))

(event Custom|OnTakeAnyDamage_Event
  (params (DamagedActor :type Actor%20Object%20Reference) (Damage :type Float%20%28single-precision%29) (DamageType :type Damage%20Type%20Object%20Reference) (InstigatedBy :type Controller%20Object%20Reference) (DamageCauser :type Actor%20Object%20Reference))
  ;[1 1 1] Damage
  (bind _output_get (Variables|Default|SetHealth (- (Variables|Default|GetHealth) Damage)))
  (Default|CallOnUpdateHealth _output_get)
  (if (< _output_get 0.0)
    (CallFunction|ReturntoRoomStart)
    (CallFunction|UseTimeMachineEnergy 1e+01 true)
    (bind _output_get_2 (Variables|Default|SetHealth 1e+02))
    (Default|CallOnUpdateHealth _output_get_2)))

(event Custom|OnEnterRoom
  (params (Room :type BP%20Room%20Segment%20Object%20Reference))
  ;[1 1 1] Entrance trigger events
  (Utilities|FlowControl|Sequence
    (:then_0
      (if (not (Utilities|Array|ContainsItem (Variables|Default|GetVisitedRooms) Room))
        (Default|OnEnterNewRoom (Variables|Default|GetBP_ExperienceComponent) (Variables|Default|GetIsInsideSafeZone) (Variables|Default|GetCurrentRoom))
        (bind _output_get (Variables|Default|SetCurrentRoom Room))
        (Utilities|Array|Add (Variables|Default|GetVisitedRooms) _output_get)))
    (:then_1
      (Variables|Default|SetIsInsideSafeZone false))))

(event Custom|OnEnterSafeZone
  ;[1 1 1] Entrance trigger events
  (Utilities|Array|Clear (Variables|Default|GetVisitedRooms))
  (Variables|Default|SetIsInsideSafeZone true)
  (Default|OnEnterSafeZone (Variables|Default|GetBP_ExperienceComponent) (Variables|Default|GetCurrentRoom)))

(event Custom|OverTimeEffects
  (if (not (Variables|Default|GetIsInsideSafeZone))
    (CallFunction|UseTimeMachineEnergy 0.75 false)))

(event Input|EnhancedActionEvents|EnhancedInputActionIA_Look
  (params (ActionValue :type Vector%202D%20Structure) (ElapsedSeconds :type Float%20%28double-precision%29) (TriggeredSeconds :type Float%20%28double-precision%29) (InputAction :type Input%20Action%20Object%20Reference :default "/Game/Input/IA_Look.IA_Look"))
  ;[1 1 1] Camera Controls
  (Pawn|Input|AddControllerYawInput (.x ActionValue))
  (Pawn|Input|AddControllerPitchInput (.y ActionValue)))

(event EventTick
  (params (DeltaSeconds :type Float%20%28single-precision%29))
  (bind _velocitytofrictioncurve (Variables|Default|GetVelocityToFrictionCurve))
  (bind _charactermovement (Variables|Character|GetCharacterMovement))
  (bind _additionalfrictionmultiplier (Variables|Default|GetAdditionalFrictionMultiplier))
  (bind _velocity (Variables|/Script/Engine.MovementComponent|GetVelocity _charactermovement))
  (bind _maxwalkspeed (Variables|/Script/Engine.CharacterMovementComponent|GetMaxWalkSpeed _charactermovement))
  (bind _returnvalue (Math|Vector|VectorLength _velocity))
  (bind _returnvalue_2 (> _returnvalue 0.01))
  (bind _returnvalue_3 (Math|Float|SelectFloat _returnvalue 0.01 _returnvalue_2))
  (bind _returnvalue_4 (/ _maxwalkspeed _returnvalue_3))
  (bind _returnvalue_5 (Math|Float|Clamp(Float) _returnvalue_4))
  (bind _returnvalue_6 (Class|KismetMathLibrary|GetRuntimeFloatCurveValue _velocitytofrictioncurve _returnvalue_5 1.0))
  (bind _returnvalue_7 (* _returnvalue_6 _additionalfrictionmultiplier))
  ;[1 1 1] Tick
  (Variables|/Script/Engine.CharacterMovementComponent|SetGroundFriction (Variables|Character|GetCharacterMovement) (* _returnvalue_7 8.0))
  (Variables|/Script/Engine.CharacterMovementComponent|SetBrakingDecelerationWalking (Variables|Character|GetCharacterMovement) (* _returnvalue_7 (Variables|Default|GetBaseBrakingDeceleration)))
  (Utilities|FlowControl|Sequence
    (:then_0
      ;[1 1 1] Sound
      (if (and (AI|Components|NavMovement|IsMovingonGround (Variables|Character|GetCharacterMovement)) (Variables|/Game/Blueprints/Character/Player/MovementComponents/BP_SlideComponent.BP_SlideComponent_C|GetIsSliding (Variables|Default|GetBP_SlideComponent)))
        (Utilities|FlowControl|DoOnce false :!label _label
          (:Completed
            (Audio|Components|Audio|Play (Variables|Default|GetSlideAudio) 0.0)
            (goto _label_2 Reset)))
        (else
          (Utilities|FlowControl|Sequence
            (:then_0
              (Utilities|FlowControl|DoOnce false :!label _label_2
                (:Completed
                  (Class|AudioParameterControllerInterface|SetTriggerParameter (Variables|Default|GetSlideAudio) "StopSlide"))))
            (:then_1
              (Utilities|FlowControl|Sequence
                (:then_0
                  (goto _label Reset))
                (:then_1
                  (Utilities|PlaySound(else->) (Math|Float|Clamp(Float) (* (/ 1.2e+03 (Math|Vector|VectorLength (Transformation|GetVelocity))) 0.3) 0.1 0.8) "/Game/Sound/SFX/MS_PlayerFootstep.MS_PlayerFootstep" (or (Math|Boolean|ANDBoolean (AI|Components|NavMovement|IsMovingonGround (Variables|Character|GetCharacterMovement)) (> (Math|Vector|VectorLength (Transformation|GetVelocity)) 0.0) (not (Variables|/Game/Blueprints/Character/Player/MovementComponents/BP_SlideComponent.BP_SlideComponent_C|GetIsSliding (Variables|Default|GetBP_SlideComponent)))) (Variables|/Game/Blueprints/Character/Player/MovementComponents/BP_WallrunComponent.BP_WallrunComponent_C|GetIsWallrunning (Variables|Default|GetBP_WallrunComponent)))))))))))
    (:then_1
      ;[1 1 1] Teleport player when he falls
      (Utilities|IsValid (Variables|Default|GetCurrentRoom)
        (:Is%20Valid
          (if (< (.z (Transformation|GetActorLocation)) (- (.z (Transformation|GetActorLocation (Variables|Default|GetCurrentRoom))) 2e+02))
            (CallFunction|ReturntoRoomStart)
            (Default|CallOnPlayerFall)
            (CallFunction|UseTimeMachineEnergy 5.0 true)))))
    (:then_2
      ;[1 1 1] Health regen
      (bind _output_get (Variables|Default|SetHealth (Math|Float|Clamp(Float) (+ (Variables|Default|GetHealth) (* (Utilities|Time|GetWorldDeltaSeconds) 5.0)) 0.0 1e+02)))
      (Default|CallOnUpdateHealth _output_get))))

(event EventBeginPlay
  ;[1 1 1] Input System Init
  (Utilities|FlowControl|Sequence
    (:then_0
      ;[1 1 1] Init Values
      (Variables|Default|SetHealth 1e+02)
      (Variables|DefaultUpgradeValues|SetDefaultMaxWalkSpeed (Variables|/Script/Engine.CharacterMovementComponent|GetMaxWalkSpeed (Variables|Character|GetCharacterMovement)))
      (Variables|DefaultUpgradeValues|SetDefaultAirControl (Variables|/Script/Engine.CharacterMovementComponent|GetAirControl (Variables|Character|GetCharacterMovement)))
      (Variables|DefaultUpgradeValues|SetDefaultJumpVelocity (Variables|/Script/Engine.CharacterMovementComponent|GetJumpZVelocity (Variables|Character|GetCharacterMovement)))
      (Variables|DefaultUpgradeValues|SetDefaultAcceleration (Variables|/Script/Engine.CharacterMovementComponent|GetMaxAcceleration (Variables|Character|GetCharacterMovement))))
    (:then_1
      (bind _asplayer_controller (Utilities|Casting|CastToPlayerController (Pawn|GetController)))
      (Input|AddMappingContext (PlayerController|LocalPlayerSubsystems|GetEnhancedInputLocalPlayerSubsystem _asplayer_controller) "/Game/Input/IMC_PlayerMappings.IMC_PlayerMappings" 0 "(bIgnoreAllPressedKeysUntilRelease=True,bForceImmediately=False,bNotifyUserSettings=False)")
      (CallFunction|InitMovementMap)
      (Utilities|Time|SetTimerbyEvent (EventDispatchers|CreateEvent :!event Custom|OverTimeEffects) 5.0 true)
      (CallFunction|InitializeSaves))
    (:then_2
      (EventDispatchers|BindEventtoOnTakeAnyDamage (delegate Custom|OnTakeAnyDamage_Event))
      (Utilities|FlowControl|Delay 5.0)
      (Default|UnlockNote (Variables|Default|GetBP_LoreComponent) "/Game/DataAssets/Notes/DA_PlayerNote_OnStart.DA_PlayerNote_OnStart")
      (if (Variables|Default|GetHasDied)
        (Default|UnlockNote (Variables|Default|GetBP_LoreComponent) "/Game/DataAssets/Notes/DA_PlayerNote_AfterRestart.DA_PlayerNote_AfterRestart")))))

(fn ConstructionScript)

(fn CanJumpInternal
  (bind _returnvalue (|CallParentFunction))
  (if _returnvalue
    (return true)
    (else
      (return (AI|Components|NavMovement|IsMovingonGround (Variables|Character|GetCharacterMovement))))))

(fn UnlockMovementAbility
  (params (Id :type String))
  (bind _movementcomponentmap (Variables|Default|GetMovementComponentMap))
  (bind (_value _returnvalue) (Utilities|Map|Find _movementcomponentmap Id))
  (if _returnvalue
    (Variables|/Game/Blueprints/Character/Player/MovementComponents/BP_MovementComponent.BP_MovementComponent_C|SetIsUnlocked _value true)))

(fn GetUnlockedAbilities
  (bind _values (Utilities|Map|Values (Variables|Default|GetMovementComponentMap)))
  (for _array_element _values
    (if (Variables|/Game/Blueprints/Character/Player/MovementComponents/BP_MovementComponent.BP_MovementComponent_C|GetIsUnlocked _array_element)
      (Utilities|Array|Add (LocalVariables|GetUnlocked) (Variables|/Game/DataAssets/Base/BP_MovementDataAsset.BP_MovementDataAsset_C|GetId (Variables|/Game/Blueprints/Character/Player/MovementComponents/BP_MovementComponent.BP_MovementComponent_C|GetData _array_element)))))
  (return (LocalVariables|GetUnlocked)))

(fn InitMovementMap
  (for _array_element (Actor|GetComponentsByClass "/Game/Blueprints/Character/Player/MovementComponents/BP_MovementComponent.BP_MovementComponent_C")
    (Utilities|Map|Add (Variables|Default|GetMovementComponentMap) (Variables|/Game/DataAssets/Base/BP_MovementDataAsset.BP_MovementDataAsset_C|GetId (Variables|/Game/Blueprints/Character/Player/MovementComponents/BP_MovementComponent.BP_MovementComponent_C|GetData _array_element)) _array_element)))

(fn UseTimeMachineEnergy
  (params (Amount :type Float%20%28double-precision%29) (IsAfterDeath :type Boolean))
  (bind _output_get (Variables|Default|SetTimeMachineEnergy (Math|Float|Clamp(Float) (- (Variables|Default|GetTimeMachineEnergy) Amount) 0.0 1e+02)))
  (Default|CallOnUpdateTimeMachineEnergy _output_get)
  (if (and (< (Variables|Default|GetTimeMachineEnergy) 0.1) IsAfterDeath)
    (Variables|Default|SetHasDied true)
    (CallFunction|SaveGame)
    (Game|OpenLevel(byName) "MainMap")))

(fn ReturntoRoomStart
  (bind _currentroom (Variables|Default|GetCurrentRoom))
  (Transformation|SetActorLocation (+ (Transformation|GetActorLocation _currentroom) "0.000000,0.000000,100.000000") false true)
  (Pawn|SetControlRotation (Pawn|GetController) (Transformation|GetActorRotation _currentroom)))

(fn AddTimeMachineEnergy
  (params (Amount :type Float%20%28double-precision%29))
  (bind _output_get (Variables|Default|SetTimeMachineEnergy (Math|Float|Clamp(Float) (+ Amount (Variables|Default|GetTimeMachineEnergy)) 0.0 1e+02)))
  (Default|CallOnUpdateTimeMachineEnergy _output_get))

(fn InitializeSaves
  (bind _returnvalue (SaveGame|DoesSaveGameExist "main"))
  (if _returnvalue
    (bind _returnvalue_2 (SaveGame|LoadGamefromSlot "main"))
    (bind _asbp_save_game (Utilities|Casting|CastToBP_SaveGame _returnvalue_2))
    (bind _output_get (Variables|Default|SetGameSaveBP _asbp_save_game))
    (Variables|/Game/Blueprints/Character/Player/BP_LoreComponent.BP_LoreComponent_C|SetUnlockedNotes (Variables|Default|GetBP_LoreComponent) (Variables|/Game/Blueprints/BP_SaveGame.BP_SaveGame_C|GetUnlockedNotes _output_get))
    (Variables|/Game/Blueprints/Character/Player/BP_LoreComponent.BP_LoreComponent_C|SetCurrentLaboratoryNoteIndex (Variables|Default|GetBP_LoreComponent) (Variables|/Game/Blueprints/BP_SaveGame.BP_SaveGame_C|GetLabNoteIndex (Variables|Default|GetGameSaveBP)))
    (Variables|Default|SetHasDied (Variables|/Game/Blueprints/BP_SaveGame.BP_SaveGame_C|GetHasDied (Variables|Default|GetGameSaveBP)))
    (Variables|/Game/Blueprints/Character/Player/BP_ExperienceComponent.BP_ExperienceComponent_C|SetOverallBestTimer (Variables|Default|GetBP_ExperienceComponent) (Variables|/Game/Blueprints/BP_SaveGame.BP_SaveGame_C|GetBestTime (Variables|Default|GetGameSaveBP)))
    (else
      (bind _returnvalue_3 (SaveGame|CreateSaveGameObject "/Game/Blueprints/BP_SaveGame.BP_SaveGame_C"))
      (bind _output_get_2 (Variables|Default|SetGameSaveBP _returnvalue_3))
      (bind _outsave (CallFunction|WritetoSaveObject _output_get_2))
      (SaveGame|SaveGametoSlot _outsave "main"))))

(fn SaveGame
  (bind _outsave (CallFunction|WritetoSaveObject (Variables|Default|GetGameSaveBP)))
  (SaveGame|SaveGametoSlot _outsave "main"))

(fn WritetoSaveObject
  (params (InSave :type BP%20Save%20Game%20Object%20Reference))
  (Variables|/Game/Blueprints/BP_SaveGame.BP_SaveGame_C|SetUnlockedNotes InSave (Variables|/Game/Blueprints/Character/Player/BP_LoreComponent.BP_LoreComponent_C|GetUnlockedNotes (Variables|Default|GetBP_LoreComponent)))
  (Variables|/Game/Blueprints/BP_SaveGame.BP_SaveGame_C|SetLabNoteIndex InSave (Variables|/Game/Blueprints/Character/Player/BP_LoreComponent.BP_LoreComponent_C|GetCurrentLaboratoryNoteIndex (Variables|Default|GetBP_LoreComponent)))
  (Variables|/Game/Blueprints/BP_SaveGame.BP_SaveGame_C|SetHasDied InSave (Variables|Default|GetHasDied))
  (Variables|/Game/Blueprints/BP_SaveGame.BP_SaveGame_C|SetBestTime InSave (Variables|/Game/Blueprints/Character/Player/BP_ExperienceComponent.BP_ExperienceComponent_C|GetOverallBestTimer (Variables|Default|GetBP_ExperienceComponent)))
  (return InSave))