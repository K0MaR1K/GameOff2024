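; BP_LoreComponent is a player character component that tracks and unlocks lore notes.
; It binds to the player's fall event to unlock a one-time note after the first fall, while UnlockLaboratoryNote hands out laboratory notes sequentially from an array.
; Both routes go through UnlockNote, which skips duplicates, records the note, broadcasts OnNoteUnlocked and saves the game through the player character.
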(event Custom|OnFall
  (if (not (Variables|Default|GetHasFallenBefore))
    (Variables|Default|SetHasFallenBefore true)
    (CallFunction|UnlockNote "/Game/DataAssets/Notes/DA_PlayerNote_AfterFirstFall.DA_PlayerNote_AfterFirstFall")))

(event EventBeginPlay
  (bind _asbp_player_character (Utilities|Casting|CastToBP_PlayerCharacter (Components|GetOwner)))
  (bind _output_get (Variables|Default|SetPlayerCharacter _asbp_player_character))
  (EventDispatchers|BindEventtoOnPlayerFall _output_get (EventDispatchers|CreateEvent :!event Custom|OnFall)))

(fn UnlockNote
  (params (Note :type BP%20Lore%20Note%20Object%20Reference))
  (if (not (Utilities|Array|ContainsItem (Variables|Default|GetUnlockedNotes) Note))
    (Utilities|Array|Add (Variables|Default|GetUnlockedNotes) Note)
    (Default|CallOnNoteUnlocked Note)
    (Default|SaveGame (Variables|Default|GetPlayerCharacter))))

(fn UnlockLaboratoryNote
  (bind _currentlaboratorynoteindex (Variables|Default|GetCurrentLaboratoryNoteIndex))
  (if (< (Variables|Default|GetCurrentLaboratoryNoteIndex) (Utilities|Array|Length (Variables|Default|GetLaboratoryNotes)))
    (LocalVariables|SetNoteIndexTemp _currentlaboratorynoteindex)
    (Math|Integer|IncrementInt _currentlaboratorynoteindex
      (:%20%20
        (CallFunction|UnlockNote (Utilities|Array|Get(acopy) (Variables|Default|GetLaboratoryNotes) (LocalVariables|GetNoteIndexTemp)))))))