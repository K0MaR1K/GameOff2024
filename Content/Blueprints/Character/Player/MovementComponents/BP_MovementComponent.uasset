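; Base player movement component that provides a start and end interface, apparently for child movement components to implement.
; On BeginPlay it casts its owner to BP_PlayerCharacter and caches the character and its CharacterMovement component.
; TryExecuteStart and TryExecuteEnd call ExecuteStart and ExecuteEnd only when IsUnlocked is true, and both Execute events are empty here.
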(event Custom|TryExecuteStart
  (if (Variables|Default|GetIsUnlocked)
    (CallFunction|ExecuteStart)))

(event Custom|ExecuteStart)

(event Custom|TryExecuteEnd
  (if (Variables|Default|GetIsUnlocked)
    (CallFunction|ExecuteEnd)))

(event Custom|ExecuteEnd)

(event EventBeginPlay
  (bind _asbp_player_character (Utilities|Casting|CastToBP_PlayerCharacter (Components|GetOwner)))
  (bind _output_get (Variables|Default|SetPlayerCharacter _asbp_player_character))
  (Variables|Default|SetCharacterMovement (Variables|/Script/Engine.Character|GetCharacterMovement _output_get)))