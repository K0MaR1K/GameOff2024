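; Player dash ability component that propels the character along the camera's aim when the dash input starts, limited by a cooldown.
; Tick runs both timers and, during a dash, overrides movement velocity with curve-scaled strength, never dropping below the forward speed captured at dash start.
; Start and cancel route through the parent's TryExecute flow, and cancelling clears the force timer.
; The upgrade system's dash distance upgrade recalculates dash strength.
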(event Custom|OnUpgradeApplied
  (params (Upgrade :type BP%20Base%20Upgrade%20Data%20Asset%20Object%20Reference) (NewValue :type Integer))
  (if (Utilities|Enum|Equal(Enum) (Variables|/Game/DataAssets/Base/BP_BaseUpgradeDataAsset.BP_BaseUpgradeDataAsset_C|GetId Upgrade) "dash_distance")
    (bind _asbp_parameter_upgrade_data_asset (Utilities|Casting|CastToBP_ParameterUpgradeDataAsset Upgrade))
    (Variables|Default|SetDashStrength (Default|CalculateUpgradedValue _asbp_parameter_upgrade_data_asset NewValue (Variables|Default|GetDefaultDashStrength)))))

(event Custom|Cancel
  (CallFunction|TryExecuteEnd))

(event Input|EnhancedActionEvents|EnhancedInputActionIA_Dash
  (params (ActionValue :type Boolean) (ElapsedSeconds :type Float%20%28double-precision%29) (TriggeredSeconds :type Float%20%28double-precision%29) (InputAction :type Input%20Action%20Object%20Reference :default "/Game/Input/IA_Dash.IA_Dash"))
  (:Started
    (CallFunction|TryExecuteStart)))

(event EventExecuteEnd
  (Variables|Default|SetDashForceTimer 0.0))

(event EventBeginPlay
  (|CallParentFunction)
  (EventDispatchers|BindEventtoOnUpgradeApplied (Variables|/Game/Blueprints/Character/Player/BP_PlayerCharacter.BP_PlayerCharacter_C|GetBP_UpgradeSystemComponent (Variables|Default|GetPlayerCharacter)) (delegate Custom|OnUpgradeApplied)))

(event EventExecuteStart
  (bind _playercharacter (Variables|Default|GetPlayerCharacter))
  (bind _returnvalue (Pawn|GetControlRotation _playercharacter :!class /Script/Engine.Pawn))
  (bind _returnvalue_2 (Math|Vector|GetForwardVector _returnvalue))
  (if (<= (Variables|Default|GetDashCooldownTimer) 0.0)
    (Variables|Default|SetOldVelocity (/ (Math|Vector|DotProduct _returnvalue_2 (Variables|/Script/Engine.MovementComponent|GetVelocity (Variables|Default|GetCharacterMovement))) (Math|Vector|VectorLength _returnvalue_2)))
    (Variables|Default|SetDashForceTimer (Variables|Default|GetDashForceTimeMax))
    (Variables|Default|SetDashCooldownTimer (Variables|Default|GetDashCooldownMax))
    (Default|DashTriggered (Variables|Default|GetPlayerCharacter))))

(event EventTick
  (params (DeltaSeconds :type Float%20%28single-precision%29))
  (bind _playercharacter (Variables|Default|GetPlayerCharacter))
  (bind _returnvalue (Pawn|GetControlRotation _playercharacter :!class /Script/Engine.Pawn))
  (bind _returnvalue_2 (Math|Vector|GetForwardVector _returnvalue))
  (Utilities|FlowControl|Sequence
    (:then_0
      (if (> (Variables|Default|GetDashCooldownTimer) 0.0)
        (Variables|Default|SetDashCooldownTimer (Math|Float|Clamp(Float) (- (Variables|Default|GetDashCooldownTimer) DeltaSeconds) 0.0 (Variables|Default|GetDashCooldownMax)))))
    (:then_1
      (if (> (Variables|Default|GetDashForceTimer) 0.0)
        (Utilities|FlowControl|Sequence
          (:then_0
            (Variables|/Script/Engine.MovementComponent|SetVelocity (Variables|Default|GetCharacterMovement) (Math|Vector|SelectVector (* _returnvalue_2 (Variables|Default|GetDashStrength) (Class|KismetMathLibrary|GetRuntimeFloatCurveValue (Variables|Default|GetDashCurve) (/ (Variables|Default|GetDashForceTimer) (Variables|Default|GetDashForceTimeMax)) 0.0)) (* _returnvalue_2 (Variables|Default|GetOldVelocity)) (> (Math|Vector|VectorLength (* _returnvalue_2 (Variables|Default|GetDashStrength) (Class|KismetMathLibrary|GetRuntimeFloatCurveValue (Variables|Default|GetDashCurve) (/ (Variables|Default|GetDashForceTimer) (Variables|Default|GetDashForceTimeMax)) 0.0))) (Variables|Default|GetOldVelocity)))))
          (:then_1
            (Variables|Default|SetDashForceTimer (Math|Float|Clamp(Float) (- (Variables|Default|GetDashForceTimer) DeltaSeconds) 0.0 (Variables|Default|GetDashForceTimeMax)))))))))