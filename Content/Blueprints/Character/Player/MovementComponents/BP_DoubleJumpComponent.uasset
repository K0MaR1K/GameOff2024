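; Player movement component that handles the double jump.
; The jump input calls TryExecuteStart, and the ExecuteStart event calls Jump on the character only while it is airborne and not wallrunning.
; A separate ExecuteJump function, not called within this graph, also jumps and cancels the dash component when its force timer is below a short threshold.
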(event Input|EnhancedActionEvents|EnhancedInputActionIA_Jump
  (params (ActionValue :type Boolean) (ElapsedSeconds :type Float%20%28double-precision%29) (TriggeredSeconds :type Float%20%28double-precision%29) (InputAction :type Input%20Action%20Object%20Reference :default "/Game/Input/IA_Jump.IA_Jump"))
  (:Started
    (CallFunction|TryExecuteStart)))

(event EventBeginPlay
  (|CallParentFunction))

(event EventExecuteStart
  (if (and (not (AI|Components|NavMovement|IsMovingonGround (Variables|Default|GetCharacterMovement))) (not (Variables|/Game/Blueprints/Character/Player/MovementComponents/BP_WallrunComponent.BP_WallrunComponent_C|GetIsWallrunning (Variables|/Game/Blueprints/Character/Player/BP_PlayerCharacter.BP_PlayerCharacter_C|GetBP_WallrunComponent (Variables|Default|GetPlayerCharacter)))))
    (Character|Jump (Variables|Default|GetPlayerCharacter))))

(fn ExecuteJump
  (bind _playercharacter (Variables|Default|GetPlayerCharacter))
  (bind _bp_dashcomponent (Variables|/Game/Blueprints/Character/Player/BP_PlayerCharacter.BP_PlayerCharacter_C|GetBP_DashComponent _playercharacter))
  (Character|Jump _playercharacter)
  (if (< (Variables|/Game/Blueprints/Character/Player/MovementComponents/BP_DashComponent.BP_DashComponent_C|GetDashForceTimer _bp_dashcomponent) 0.1)
    (Default|Cancel _bp_dashcomponent)))