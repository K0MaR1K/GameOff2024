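; Player movement component that adds unlockable wallrunning, with jump-off, crouch release and camera roll.
; Each tick it traces right and left for valid walls while the player falls and presses forward, cancels dashes and drives motion through LaunchCharacter.
; A timer, extendable by upgrades, holds height via Z-velocity override, then gravity eases toward a wallrun value.
; Ending a run restores gravity and briefly suppresses reattachment.
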(event Custom|OnUpgradeApplied
  (params (Upgrade :type BP%20Base%20Upgrade%20Data%20Asset%20Object%20Reference) (NewValue :type Integer))
  (if (Utilities|Enum|Equal(Enum) (Variables|/Game/DataAssets/Base/BP_BaseUpgradeDataAsset.BP_BaseUpgradeDataAsset_C|GetId Upgrade) "wallrun_duration")
    (bind _asbp_parameter_upgrade_data_asset (Utilities|Casting|CastToBP_ParameterUpgradeDataAsset Upgrade))
    (Variables|Default|SetMaxWallrunDuration (Default|CalculateUpgradedValue _asbp_parameter_upgrade_data_asset NewValue (Variables|Default|GetDefaultMaxWallrunDuration)))))

(event Custom|ResetWallrunSupression
  (Variables|Default|SetIsWallrunSupressed false)
  (Utilities|Time|ClearTimerbyFunctionName 0 "ResetWallrunSupression"))

(event Input|EnhancedActionEvents|EnhancedInputActionIA_Jump
  (params (ActionValue :type Boolean) (ElapsedSeconds :type Float%20%28double-precision%29) (TriggeredSeconds :type Float%20%28double-precision%29) (InputAction :type Input%20Action%20Object%20Reference :default "/Game/Input/IA_Jump.IA_Jump"))
  (bind _wallrunnormal (Variables|Default|GetWallrunNormal))
  (bind _wallrunjumpoffforce (Variables|Default|GetWallrunJumpOffForce))
  (bind _returnvalue (* _wallrunnormal _wallrunjumpoffforce))
  (:Started
    (if (Variables|Default|GetIsWallrunning)
      (CallFunction|EndWallrun)
      (Character|LaunchCharacter (Variables|Default|GetPlayerCharacter) (Math|Vector|MakeVector (.x _returnvalue) (.y _returnvalue) (Variables|Default|GetWallrunJumpHeight)) false true))))

(event Input|EnhancedActionEvents|EnhancedInputActionIA_Move
  (params (ActionValue :type Vector%202D%20Structure) (ElapsedSeconds :type Float%20%28double-precision%29) (TriggeredSeconds :type Float%20%28double-precision%29) (InputAction :type Input%20Action%20Object%20Reference :default "/Game/Input/IA_Move.IA_Move"))
  (:Triggered
    (Variables|Default|SetIsPressingForward (> (.y ActionValue) 0.0) :!label _label))
  (:Completed
    (goto _label)))

(event Input|EnhancedActionEvents|EnhancedInputActionIA_Crouch
  (params (ActionValue :type Boolean) (ElapsedSeconds :type Float%20%28double-precision%29) (TriggeredSeconds :type Float%20%28double-precision%29) (InputAction :type Input%20Action%20Object%20Reference :default "/Game/Input/IA_Crouch.IA_Crouch"))
  (if (Variables|Default|GetIsWallrunning)
    (CallFunction|EndWallrun)))

(event EventBeginPlay
  (|CallParentFunction)
  (Variables|Default|SetDefaultGravity (Variables|/Script/Engine.CharacterMovementComponent|GetGravityScale (Variables|Default|GetCharacterMovement)))
  (EventDispatchers|BindEventtoOnUpgradeApplied (Variables|/Game/Blueprints/Character/Player/BP_PlayerCharacter.BP_PlayerCharacter_C|GetBP_UpgradeSystemComponent (Variables|Default|GetPlayerCharacter)) (delegate Custom|OnUpgradeApplied)))

(event EventTick
  (params (DeltaSeconds :type Float%20%28single-precision%29))
  (bind (_right _left) (Utilities|WallrunEndVectors))
  (if (Variables|Default|GetIsUnlocked)
    (CallFunction|CameraTick)
    (bind _onwall (CallFunction|WallrunMovement (Transformation|GetActorLocation (Variables|Default|GetPlayerCharacter)) _right -1.0))
    (if _onwall
      (CallFunction|StartWallrun)
      (Variables|Default|SetIsWallrunningOnRight true)
      (Utilities|FlowControl|Sequence :!label _label
        (:then_0
          (Default|Cancel (Variables|/Game/Blueprints/Character/Player/BP_PlayerCharacter.BP_PlayerCharacter_C|GetBP_DashComponent (Variables|Default|GetPlayerCharacter)))
          (if (> (Variables|Default|GetWallrunTimer) 0.0)
            (Variables|Default|SetWallrunTimer (- (Variables|Default|GetWallrunTimer) (Utilities|Time|GetWorldDeltaSeconds)))
            (else
              (Variables|Default|SetRemoveGravity false))))
        (:then_1
          (if (not (Variables|Default|GetRemoveGravity))
            (Variables|/Script/Engine.CharacterMovementComponent|SetGravityScale (Variables|Default|GetCharacterMovement) (Math|Interpolation|FInterpTo (Variables|/Script/Engine.CharacterMovementComponent|GetGravityScale (Variables|Default|GetCharacterMovement)) (Variables|Default|GetWallrunTargetGravity) (Utilities|Time|GetWorldDeltaSeconds) 1e+01)))))
      (elif (Variables|Default|GetIsWallrunningOnRight)
        (CallFunction|EndWallrun)
        (else
          (bind _onwall_2 (CallFunction|WallrunMovement (Transformation|GetActorLocation (Variables|Default|GetPlayerCharacter)) _left 1.0))
          (if _onwall_2
            (CallFunction|StartWallrun)
            (Variables|Default|SetIsWallrunningOnRight false)
            (goto _label)
            (else
              (CallFunction|EndWallrun))))))))

(fn WallrunMovement
  (params (Start :type Vector) (End :type Vector) (WallrunDirection :type Float%20%28double-precision%29))
  (bind _playercharacter (Variables|Default|GetPlayerCharacter))
  (bind _returnvalue (Pawn|GetControlRotation _playercharacter :!class /Script/Engine.Pawn))
  (bind _outhit (Collision|LineTraceByChannel Start End "TraceTypeQuery1" false 0 "None"))
  (if (Math|Boolean|ANDBoolean (or (> (.pitch _returnvalue) 315.0) (< (.pitch _returnvalue) 45.0)) (AI|Components|NavMovement|IsFalling (Variables|Default|GetCharacterMovement)) (.bblockinghit _outhit) (Utilities|IsValidWallRunVector (.normal _outhit)) (Variables|Default|GetIsPressingForward) (not (Variables|Default|GetIsWallrunSupressed)))
    (Variables|Default|SetWallrunNormal (.normal _outhit))
    (Character|LaunchCharacter (Variables|Default|GetPlayerCharacter) (Utilities|PlayertoWallVector) false false) ; Stick to wall
    (Character|LaunchCharacter (Variables|Default|GetPlayerCharacter) (* (Math|Vector|CrossProduct (Variables|Default|GetWallrunNormal) "0.000000,0.000000,1.000000") (* WallrunDirection (Variables|Default|GetWallrunSpeed))) true (Variables|Default|GetRemoveGravity)) ; Move forward
    (return true)
    (else
      (return false))))

(fn EndWallrun
  (if (Variables|Default|GetIsWallrunning)
    (Variables|Default|SetIsWallrunning false)
    (Variables|Default|SetIsWallrunningOnRight false)
    (Variables|/Script/Engine.CharacterMovementComponent|SetGravityScale (Variables|Default|GetCharacterMovement) (Variables|Default|GetDefaultGravity))
    (CallFunction|SupressWallrun)
    (Pawn|Components|CharacterMovement|SetMovementMode (Variables|Default|GetCharacterMovement) "MOVE_Falling" 0)
    (Variables|Default|SetWallrunTimer 0.0)))

(fn SupressWallrun
  (Variables|Default|SetIsWallrunSupressed true)
  (Utilities|Time|SetTimerbyFunctionName 0 "ResetWallrunSupression" (Variables|Default|GetResetTime)))

(fn CameraTick
  (if (Variables|Default|GetIsWallrunning)
    (if (Variables|Default|GetIsWallrunningOnRight)
      (CallFunction|CameraTilt -15.0)
      (else
        (CallFunction|CameraTilt 15.0)))
    (else
      (CallFunction|CameraTilt 0.0))))

(fn CameraTilt
  (params (TargetRoll :type Float%20%28double-precision%29))
  (bind _playercharacter (Variables|Default|GetPlayerCharacter))
  (bind _returnvalue (Pawn|GetControlRotation _playercharacter :!class /Script/Engine.Pawn))
  (bind (_roll _pitch _yaw) (Math|Rotator|BreakRotator _returnvalue))
  (Pawn|SetControlRotation (Pawn|GetController (Variables|Default|GetPlayerCharacter)) (Math|Interpolation|RInterpTo _returnvalue (Math|Rotator|MakeRotator TargetRoll _pitch _yaw) (Utilities|Time|GetWorldDeltaSeconds) 1e+01)))

(fn StartWallrun
  (if (not (Variables|Default|GetIsWallrunning))
    (Variables|Default|SetIsWallrunning true)
    (Variables|Default|SetWallrunTimer (Variables|Default|GetMaxWallrunDuration))
    (Variables|Default|SetRemoveGravity true)))