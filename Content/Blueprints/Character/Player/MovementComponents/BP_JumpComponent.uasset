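; Player movement component that handles jumping with input buffering, driven by the IA_Jump input action.
; A press jumps immediately when grounded, otherwise starts a buffer timer that Tick counts down, jumping if the player lands before it expires.
; Each jump plays a 2D sound and cancels the dash component when its force timer is below a small threshold.
; Input Started and Canceled route through TryExecuteStart and TryExecuteEnd, with ending calling StopJumping.
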(event Input|EnhancedActionEvents|EnhancedInputActionIA_Jump
  (params (ActionValue :type Boolean) (ElapsedSeconds :type Float%20%28double-precision%29) (TriggeredSeconds :type Float%20%28double-precision%29) (InputAction :type Input%20Action%20Object%20Reference :default "/Game/Input/IA_Jump.IA_Jump"))
  (:Started
    (CallFunction|TryExecuteStart))
  (:Canceled
    (CallFunction|TryExecuteEnd)))

(event EventBeginPlay
  (|CallParentFunction))

(event EventExecuteEnd
  (Character|StopJumping (Variables|Default|GetPlayerCharacter)))

(event EventExecuteStart
  (if (AI|Components|NavMovement|IsMovingonGround (Variables|Default|GetCharacterMovement))
    (CallFunction|ExecuteJump)
    (else
      (Variables|Default|SetJumpBufferTimer (Variables|Default|GetJumpBufferMax)))))

(event EventTick
  (params (DeltaSeconds :type Float%20%28single-precision%29))
  (if (> (Variables|Default|GetJumpBufferTimer) 0.0)
    (Utilities|FlowControl|Sequence
      (:then_0
        (if (AI|Components|NavMovement|IsMovingonGround (Variables|Default|GetCharacterMovement))
          (CallFunction|ExecuteJump)
          (Variables|Default|SetJumpBufferTimer 0.0)))
      (:then_1
        (Variables|Default|SetJumpBufferTimer (Math|Float|Clamp(Float) (- (Variables|Default|GetJumpBufferTimer) DeltaSeconds) 0.0 (Variables|Default|GetJumpBufferMax)))))))

(fn ExecuteJump
  (bind _playercharacter (Variables|Default|GetPlayerCharacter))
  (bind _bp_dashcomponent (Variables|/Game/Blueprints/Character/Player/BP_PlayerCharacter.BP_PlayerCharacter_C|GetBP_DashComponent _playercharacter))
  (Character|Jump _playercharacter)
  (Audio|PlaySound2D "/Game/Sound/SFX/MS_Jump.MS_Jump" 1.0 1.0 0.0 0 0)
  (if (< (Variables|/Game/Blueprints/Character/Player/MovementComponents/BP_DashComponent.BP_DashComponent_C|GetDashForceTimer _bp_dashcomponent) 0.1)
    (Default|Cancel _bp_dashcomponent)))