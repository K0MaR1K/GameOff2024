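; BP_RightComponent is a player movement component that moves the character to the right.
; Positive X values from the IA_Move input action are stored as the scale, then TryExecuteStart is called.
; ExecuteStart applies movement input along the right vector of the control rotation's yaw, ignoring pitch and roll.
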(event Input|EnhancedActionEvents|EnhancedInputActionIA_Move
  (params (ActionValue :type Vector%202D%20Structure) (ElapsedSeconds :type Float%20%28double-precision%29) (TriggeredSeconds :type Float%20%28double-precision%29) (InputAction :type Input%20Action%20Object%20Reference :default "/Game/Input/IA_Move.IA_Move"))
  (:Triggered
    (if (> (.x ActionValue) 0.0)
      (Variables|Default|SetScale%20Value (.x ActionValue))
      (CallFunction|TryExecuteStart))))

(event EventBeginPlay
  (|CallParentFunction))

(event EventExecuteStart
  (Pawn|Input|AddMovementInput (Variables|Default|GetPlayerCharacter) (Math|Vector|GetRightVector (Math|Rotator|MakeRotator 0.0 0.0 (.yaw (Pawn|GetControlRotation (Variables|Default|GetPlayerCharacter) :!class /Script/Engine.Pawn)))) (Variables|Default|GetScale%20Value) false))