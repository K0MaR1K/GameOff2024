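; Player movement component that adds a crouch slide with a stamina-limited speed boost.
; Crouch input cancels any dash and launches the player along horizontal velocity if grounded with over half stamina.
; When unlocked, Tick starts sliding while crouched at speed by lowering friction, ends it when slow, and drains or regenerates stamina.
; The slide_velocity upgrade recalculates boost force through the upgrade system's event.
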(event Custom|OnUpgradeApplied
  (params (Upgrade :type BP%20Base%20Upgrade%20Data%20Asset%20Object%20Reference) (NewValue :type Integer))
  (if (Utilities|Enum|Equal(Enum) (Variables|/Game/DataAssets/Base/BP_BaseUpgradeDataAsset.BP_BaseUpgradeDataAsset_C|GetId Upgrade) "slide_velocity")
    (bind _asbp_parameter_upgrade_data_asset (Utilities|Casting|CastToBP_ParameterUpgradeDataAsset Upgrade))
    (Variables|Default|SetSlideForce (Default|CalculateUpgradedValue _asbp_parameter_upgrade_data_asset NewValue (Variables|Default|GetDefaultSlideForce)))))

(event Input|EnhancedActionEvents|EnhancedInputActionIA_Crouch
  (params (ActionValue :type Boolean) (ElapsedSeconds :type Float%20%28double-precision%29) (TriggeredSeconds :type Float%20%28double-precision%29) (InputAction :type Input%20Action%20Object%20Reference :default "/Game/Input/IA_Crouch.IA_Crouch"))
  (:Started
    (CallFunction|TryExecuteStart))
  (:Completed
    (CallFunction|TryExecuteEnd)))

(event EventBeginPlay
  (|CallParentFunction)
  (EventDispatchers|BindEventtoOnUpgradeApplied (Variables|/Game/Blueprints/Character/Player/BP_PlayerCharacter.BP_PlayerCharacter_C|GetBP_UpgradeSystemComponent (Variables|Default|GetPlayerCharacter)) (delegate Custom|OnUpgradeApplied)))

(event EventExecuteStart
  (Default|Cancel (Variables|/Game/Blueprints/Character/Player/BP_PlayerCharacter.BP_PlayerCharacter_C|GetBP_DashComponent (Variables|Default|GetPlayerCharacter)))
  (CallFunction|TryPerformSlideBoost))

(event EventTick
  (params (DeltaSeconds :type Float%20%28single-precision%29))
  (if (Variables|Default|GetIsUnlocked)
    (Utilities|FlowControl|Sequence
      (:then_0
        (if (Variables|Default|GetIsSliding)
          (Utilities|FlowControl|Sequence
            (:then_0
              (if (< (Math|Vector|VectorLength (Variables|/Script/Engine.MovementComponent|GetVelocity (Variables|Default|GetCharacterMovement))) (Variables|Default|GetRequiredSlideVelocity))
                (CallFunction|EndSlide)))
            (:then_1
              (Variables|Default|SetSlideStamina (Math|Float|Clamp(Float) (- (Variables|Default|GetSlideStamina) (* DeltaSeconds 2.0)) 0.0 (Variables|Default|GetSlideStaminaMax)))))
          (elif (and (AI|Components|NavMovement|IsCrouching (Variables|Default|GetCharacterMovement)) (> (Math|Vector|VectorLength (Variables|/Script/Engine.MovementComponent|GetVelocity (Variables|Default|GetCharacterMovement))) (Variables|Default|GetRequiredSlideVelocity)))
            (CallFunction|StartSlide))))
      (:then_1
        (if (not (AI|Components|NavMovement|IsCrouching (Variables|Default|GetCharacterMovement)))
          (Variables|Default|SetSlideStamina (Math|Float|Clamp(Float) (+ DeltaSeconds (Variables|Default|GetSlideStamina)) 0.0 (Variables|Default|GetSlideStaminaMax))))))))

(event EventExecuteEnd
  (CallFunction|EndSlide))

(fn TryPerformSlideBoost
  (bind _charactermovement (Variables|Default|GetCharacterMovement))
  (bind _velocity (Variables|/Script/Engine.MovementComponent|GetVelocity _charactermovement))
  (bind _returnvalue (Math|Vector|Normalize _velocity))
  (if (and (AI|Components|NavMovement|IsMovingonGround (Variables|Default|GetCharacterMovement)) (> (Variables|Default|GetSlideStamina) (/ (Variables|Default|GetSlideStaminaMax) 2.0)))
    (Character|LaunchCharacter (Variables|Default|GetPlayerCharacter) (* (Math|Vector|MakeVector (.x _returnvalue) (.y _returnvalue) 0.0) (Variables|Default|GetSlideForce)) false false)))

(fn EndSlide
  (Variables|/Game/Blueprints/Character/Player/BP_PlayerCharacter.BP_PlayerCharacter_C|SetAdditionalFrictionMultiplier (Variables|Default|GetPlayerCharacter) 1.0)
  (Variables|Default|SetIsSliding false))

(fn StartSlide
  (Variables|/Game/Blueprints/Character/Player/BP_PlayerCharacter.BP_PlayerCharacter_C|SetAdditionalFrictionMultiplier (Variables|Default|GetPlayerCharacter) 0.07)
  (Variables|Default|SetIsSliding true))