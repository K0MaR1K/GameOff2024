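; Player controller that turns menu-related input into UI: options menu, notes menu and upgrade selection.
; The menu key exits the current menu if allowed or opens a pausing options menu, while the notes key calls the player HUD.
; The upgrade key, when no menu is open, spends an available upgrade and offers random choices from the character's upgrade component.
; UnlockNewAbilities shows ability unlocks through the same pausing, non-key-exitable selection menu.
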(event Custom|UnlockNewAbilities
  (bind _asbp_player_character (Utilities|Casting|CastToBP_PlayerCharacter (Game|GetPlayerCharacter 0)))
  (bind _upgrades (Default|GetRandomUpgrades (Variables|/Game/Blueprints/Character/Player/BP_PlayerCharacter.BP_PlayerCharacter_C|GetBP_UpgradeSystemComponent _asbp_player_character) 2 true))
  (bind _returnvalue (UserInterface|CreateWidget "/Game/Blueprints/UI/WB_UpgradeSelectionMenu.WB_UpgradeSelectionMenu_C" 0 _upgrades))
  (Default|SetCurrentMenu (Variables|Default|GetMenuLayer) _returnvalue true false))

(event Input|EnhancedActionEvents|EnhancedInputActionIA_Menu
  (params (ActionValue :type Boolean) (ElapsedSeconds :type Float%20%28double-precision%29) (TriggeredSeconds :type Float%20%28double-precision%29) (InputAction :type Input%20Action%20Object%20Reference :default "/Game/Input/IA_Menu.IA_Menu"))
  (:Started
    (if (Default|IsMenuinUse (Variables|Default|GetMenuLayer))
      (if (Variables|/Game/Blueprints/UI/WB_MenuLayer.WB_MenuLayer_C|GetCan%20be%20Exited%20WIth%20Key (Variables|Default|GetMenuLayer))
        (Default|ExitMenus (Variables|Default|GetMenuLayer)))
      (else
        (bind _returnvalue (UserInterface|CreateWidget "/Game/Blueprints/UI/WB_OptionsMenu.WB_OptionsMenu_C"))
        (Default|SetCurrentMenu (Variables|Default|GetMenuLayer) _returnvalue true true)))))

(event Input|EnhancedActionEvents|EnhancedInputActionIA_Upgrade
  (params (ActionValue :type Boolean) (ElapsedSeconds :type Float%20%28double-precision%29) (TriggeredSeconds :type Float%20%28double-precision%29) (InputAction :type Input%20Action%20Object%20Reference :default "/Game/Input/IA_Upgrade.IA_Upgrade"))
  (:Started
    (if (not (Default|IsMenuinUse (Variables|Default|GetMenuLayer)))
      (bind _asbp_player_character (Utilities|Casting|CastToBP_PlayerCharacter (Game|GetPlayerCharacter 0)))
      (if (> (Variables|/Game/Blueprints/Character/Player/BP_UpgradeSystemComponent.BP_UpgradeSystemComponent_C|GetUpgradesAvailable (Variables|/Game/Blueprints/Character/Player/BP_PlayerCharacter.BP_PlayerCharacter_C|GetBP_UpgradeSystemComponent _asbp_player_character)) 0)
        (Default|UseUpgrade (Variables|/Game/Blueprints/Character/Player/BP_PlayerCharacter.BP_PlayerCharacter_C|GetBP_UpgradeSystemComponent _asbp_player_character))
        (bind _upgrades (Default|GetRandomUpgrades (Variables|/Game/Blueprints/Character/Player/BP_PlayerCharacter.BP_PlayerCharacter_C|GetBP_UpgradeSystemComponent _asbp_player_character) 3 false))
        (bind _returnvalue (UserInterface|CreateWidget "/Game/Blueprints/UI/WB_UpgradeSelectionMenu.WB_UpgradeSelectionMenu_C" 0 _upgrades))
        (Default|SetCurrentMenu (Variables|Default|GetMenuLayer) _returnvalue true false)))))

(event Input|EnhancedActionEvents|EnhancedInputActionIA_OpenNotes
  (params (ActionValue :type Boolean) (ElapsedSeconds :type Float%20%28double-precision%29) (TriggeredSeconds :type Float%20%28double-precision%29) (InputAction :type Input%20Action%20Object%20Reference :default "/Game/Input/IA_OpenNotes.IA_OpenNotes"))
  (:Started
    (bind _asbp_player_hud (Utilities|Casting|CastToBP_PlayerHUD (HUD|GetHUD)))
    (Default|OpenNotesMenu (Variables|/Game/Blueprints/Character/Player/BP_PlayerHUD.BP_PlayerHUD_C|GetPlayerHUD _asbp_player_hud))))

(fn ConstructionScript)