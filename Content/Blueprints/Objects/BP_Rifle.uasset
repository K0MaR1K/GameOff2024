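; BP_Rifle is a rifle actor with an animated part, shot audio and a reload motion.
; Tick swings RifleRiflePart03 back and forth in pitch using a sine of accumulated time, replaying a 2D rotation sound through a DoOnce gate reset after a sine-based delay with a minimum.
; Shoot plays the MSRifleShoot sound and restarts ReloadTimeline, which drives the root's pitch for the reload animation.
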(event Custom|Shoot
  (Audio|Components|Audio|Play (Variables|Default|GetMS_RifleShoot) 0.0)
  (bind _rotation (Timeline|ReloadTimeline PlayFromStart)
    (:Update
      (Transformation|SetRelativeRotation (Variables|Default|GetDefaultSceneRoot) (Math|Rotator|MakeRotator 0.0 _rotation 0.0) false false))))

(event EventBeginPlay
  (Variables|Default|Setrot%20speed 0.0))

(event Collision|EventActorBeginOverlap
  (params (OtherActor :type Actor%20Object%20Reference)))

(event EventTick
  (params (DeltaSeconds :type Float%20%28single-precision%29))
  (bind _rifle_rifle_part_03 (Variables|Default|Getrifle_rifle_part_03))
  (Variables|Default|Setrot%20speed (+ (Variables|Default|Getrot%20speed) DeltaSeconds))
  (Transformation|SetRelativeRotation _rifle_rifle_part_03 (Math|Rotator|CombineRotators (Variables|/Script/Engine.SceneComponent|GetRelativeRotation _rifle_rifle_part_03) (* (Math|Rotator|MakeRotator 0.0 (* (Math|Trig|Sin(Radians) (Variables|Default|Getrot%20speed)) 5e+02) 0.0) DeltaSeconds)) false false)
  (Utilities|FlowControl|DoOnce false :!label _label
    (:Completed
      (Audio|PlaySound2D "/Game/Sound/SFX/rotation.rotation" 0.06 1.0 0.0 0 0 false)
      (Utilities|FlowControl|Delay (Math|Float|Max(Float) (Math|Trig|Sin(Radians) (Variables|Default|Getrot%20speed)) 0.4))
      (goto _label Reset))))

(fn ConstructionScript)